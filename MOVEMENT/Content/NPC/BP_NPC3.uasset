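; BP_NPC3 is an NPC Blueprint that wanders around the spot where it spawned.
; On BeginPlay it stores its spawn location, waits a set delay, then starts a roam loop.
; The loop uses AI MoveTo toward a random reachable point within a radius of that location.
; Whether the move finishes or fails, it waits a random interval and picks a new point.
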(event Custom|RandomLoCATION
  (AI|AIMoveTo (AI|GetAIController self) (.RandomLocation (AI|Navigation|GetRandomReachablePointinRadius (Variables|Default|GetSpawn%20loaction) (Variables|Default|GetRadius) 0 0)) 0 -1.0 "Default" "Default" true true
    (:OnRequestFailed
      _)
    (:OnMoveFinished
      _))
  (Utilities|FlowControl|Delay (Math|Random|RandomFloatinRange (Variables|Default|GetRoamIntervalMin) (Variables|Default|GetRoamIntervalMax)))
  (CallFunction|RandomLoCATION))

(event EventBeginPlay
  (Variables|Default|SetSpawn%20loaction (Transformation|GetActorLocation))
  (Utilities|FlowControl|Delay (Variables|Default|GetDuration))
  (CallFunction|RandomLoCATION))

(fn ConstructionScript)