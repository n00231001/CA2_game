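; BP_NPC2 is an NPC Blueprint that steps through an array of dialogue lines on screen.
; Each Talk call increments Talkingdex before reading, lazily creates a WBdialouge widget for player 0, and sets its TalkText to that entry.
; Once the index exceeds the array length (checked with <=), the widget is removed from the viewport; nothing here resets the index.
; StartTalking and the construction script are empty.
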(event Custom|StartTalking)

(event EventTalk
  (Math|Integer|IncrementInt (Variables|Default|Gettalkingdex)
    (:%20%20
      (if (<= (Variables|Default|Gettalkingdex) (Utilities|Array|Length (Variables|Default|Getdialouge)))
        (Variables|Default|GetUI
          (:then
            _)
          (:else
            (bind _returnvalue (UserInterface|CreateWidget "/Game/NPC/WB-dialouge.WB-dialouge_C" (Game|GetPlayerController 0)))
            (bind _output_get (Variables|Default|SetUI _returnvalue))
            (UserInterface|Viewport|AddtoViewport _output_get 0)))
        (Rendering|Components|TextRender|SetText (Variables|/Game/NPC/WB-dialouge.WB-dialouge_C|GettalkText (Variables|Default|GetUI)) (Utilities|Text|ToText(String) (Utilities|Array|Get(acopy) (Variables|Default|Getdialouge) (Variables|Default|Gettalkingdex))))
        (else
          (Widget|RemovefromParent (Variables|Default|GetUI)))))))

(fn ConstructionScript)