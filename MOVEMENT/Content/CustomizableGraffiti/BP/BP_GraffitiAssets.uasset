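; Customizable graffiti decal actor whose texture, color, normal map, mask, placement and surface properties are exposed as variables.
; The construction script calls UpdateGraffitiDecal, which creates a dynamic material instance from DecalMaterial, pushes every variable into it and assigns it to the decal.
; Helper functions restore class defaults, randomize color, or pick a random Texture2D under GraffitiPath through the Asset Registry, then refresh the decal.
; The event graph holds no logic.
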(event EventBeginPlay)

(event Collision|EventActorBeginOverlap
  (params (OtherActor :type Actor%20Object%20Reference)))

(event EventTick
  (params (DeltaSeconds :type Float%20%28single-precision%29)))

(fn ConstructionScript
  (MaterialSettings|UpdateGraffitiDecal))

(fn UpdateGraffitiDecal
  (bind _decal (Variables|Default|GetDecal))
  (bind _maskoffset (Variables|MaterialSettings|GetMaskOffset))
  (bind _graffitioffset (Variables|MaterialSettings|GetGraffitiOffset))
  (bind (_x _y) (Math|Vector2D|BreakVector2D _graffitioffset))
  (bind (_x_2 _y_2) (Math|Vector2D|BreakVector2D _maskoffset))
  (Utilities|FlowControl|Sequence
    (:then_0
      (Rendering|Components|Decal|SetDecalMaterial _decal (Variables|MaterialSettings|GetDecalMaterial))
      (bind _returnvalue (Rendering|Material|CreateDynamicMaterialInstance _decal :!class /Script/Engine.DecalComponent))
      (Variables|Components|SetDynamicMaterial _returnvalue))
    (:then_1
      (Rendering|Material|SetScalarParameterValue (Variables|Components|GetDynamicMaterial) "DecalStretching" (Math|Conversions|ToFloat(Boolean) (Variables|MaterialSettings|GetDecalStretching)) :!class /Script/Engine.MaterialInstanceDynamic)
      (Rendering|Material|SetScalarParameterValue (Variables|Components|GetDynamicMaterial) "HueShift" (Variables|MaterialSettings|GetHueShift) :!class /Script/Engine.MaterialInstanceDynamic)
      (Rendering|Material|SetVectorParameterValue (Variables|Components|GetDynamicMaterial) "ColorMultiply" (Variables|MaterialSettings|GetColorMultiply) :!class /Script/Engine.MaterialInstanceDynamic)
      (Rendering|Material|SetScalarParameterValue (Variables|Components|GetDynamicMaterial) "Desaturation" (Variables|MaterialSettings|GetDesaturation) :!class /Script/Engine.MaterialInstanceDynamic)
      (Rendering|Material|SetTextureParameterValue (Variables|Components|GetDynamicMaterial) "Texture" (Variables|MaterialSettings|GetGraffitiTexture))
      (Rendering|Material|SetScalarParameterValue (Variables|Components|GetDynamicMaterial) "Brightness" (Variables|MaterialSettings|GetBrightness) :!class /Script/Engine.MaterialInstanceDynamic)
      (Rendering|Material|SetScalarParameterValue (Variables|Components|GetDynamicMaterial) "NormalMapUVScale" (Variables|MaterialSettings|GetNormalMapUVScale) :!class /Script/Engine.MaterialInstanceDynamic)
      (Rendering|Material|SetTextureParameterValue (Variables|Components|GetDynamicMaterial) "NormalMap" (Variables|MaterialSettings|GetNormalMapTexture))
      (Rendering|Material|SetScalarParameterValue (Variables|Components|GetDynamicMaterial) "InvertColor" (Math|Conversions|ToFloat(Boolean) (Variables|MaterialSettings|GetInvertColor)) :!class /Script/Engine.MaterialInstanceDynamic)
      (Rendering|Material|SetScalarParameterValue (Variables|Components|GetDynamicMaterial) "MaxOpacity" (Variables|MaterialSettings|GetMaxOpacity) :!class /Script/Engine.MaterialInstanceDynamic)
      (Rendering|Material|SetScalarParameterValue (Variables|Components|GetDynamicMaterial) "MaskPower" (Variables|MaterialSettings|GetMaskPower) :!class /Script/Engine.MaterialInstanceDynamic)
      (Rendering|Material|SetScalarParameterValue (Variables|Components|GetDynamicMaterial) "MaskScale" (Variables|MaterialSettings|GetMaskUVScale) :!class /Script/Engine.MaterialInstanceDynamic)
      (Rendering|Material|SetTextureParameterValue (Variables|Components|GetDynamicMaterial) "MaskTexture" (Variables|MaterialSettings|GetMaskTexture))
      (Rendering|Material|SetScalarParameterValue (Variables|Components|GetDynamicMaterial) "MaskOffsetX" _x_2 :!class /Script/Engine.MaterialInstanceDynamic)
      (Rendering|Material|SetScalarParameterValue (Variables|Components|GetDynamicMaterial) "MaskOffsetY" _y_2 :!class /Script/Engine.MaterialInstanceDynamic)
      (Rendering|Material|SetScalarParameterValue (Variables|Components|GetDynamicMaterial) "GraffitiOffsetX" _x :!class /Script/Engine.MaterialInstanceDynamic)
      (Rendering|Material|SetScalarParameterValue (Variables|Components|GetDynamicMaterial) "GraffitiOffsetY" _y :!class /Script/Engine.MaterialInstanceDynamic)
      (Rendering|Material|SetScalarParameterValue (Variables|Components|GetDynamicMaterial) "GraffitiScale" (Variables|MaterialSettings|GetGraffitiUVScale) :!class /Script/Engine.MaterialInstanceDynamic)
      (Rendering|Material|SetScalarParameterValue (Variables|Components|GetDynamicMaterial) "Roughness" (Variables|MaterialSettings|GetRoughness) :!class /Script/Engine.MaterialInstanceDynamic)
      (Rendering|Material|SetScalarParameterValue (Variables|Components|GetDynamicMaterial) "Metallic" (Variables|MaterialSettings|GetMetallic) :!class /Script/Engine.MaterialInstanceDynamic))
    (:then_2
      (Rendering|Components|Decal|SetDecalMaterial (Variables|Default|GetDecal) (Variables|Components|GetDynamicMaterial)))))

(fn ResettoDefault
  (bind (_dynamicmaterial _graffitipath _graffititexture _decalstretching _graffitioffset _graffitiuvscale _roughness _metallic _invertcolor _colormultiply _hueshift _desaturation _brightness _normalmaptexture _normalmapuvscale _maxopacity _maskpower _masktexture _maskuvscale _maskoffset) (Utilities|GetClassDefaults "BP_GraffitiAssets_C"))
  (bind (_dynamicmaterial_2 _graffitipath_2 _graffititexture_2 _decalstretching_2 _graffitioffset_2 _graffitiuvscale_2 _roughness_2 _metallic_2 _invertcolor_2 _colormultiply_2 _hueshift_2 _desaturation_2 _brightness_2 _normalmaptexture_2 _normalmapuvscale_2 _maxopacity_2 _maskpower_2 _masktexture_2 _maskuvscale_2 _maskoffset_2 _decalmaterial) (Utilities|GetClassDefaults "BP_GraffitiAssets_C"))
  (Utilities|FlowControl|Sequence
    (:then_0
      (Variables|MaterialSettings|SetDecalMaterial _decalmaterial)
      (Variables|MaterialSettings|SetGraffitiTexture _graffititexture_2)
      (Variables|MaterialSettings|SetInvertColor _invertcolor_2)
      (Variables|MaterialSettings|SetColorMultiply _colormultiply_2)
      (Variables|MaterialSettings|SetHueShift _hueshift_2)
      (Variables|MaterialSettings|SetDesaturation _desaturation_2)
      (Variables|MaterialSettings|SetBrightness _brightness_2)
      (Variables|MaterialSettings|SetNormalMapTexture _normalmaptexture_2)
      (Variables|MaterialSettings|SetNormalMapUVScale _normalmapuvscale_2)
      (Variables|MaterialSettings|SetDecalStretching _decalstretching)
      (Variables|MaterialSettings|SetMaxOpacity _maxopacity)
      (Variables|MaterialSettings|SetMaskPower _maskpower)
      (Variables|MaterialSettings|SetMaskTexture _masktexture)
      (Variables|MaterialSettings|SetMaskUVScale _maskuvscale)
      (Variables|MaterialSettings|SetMaskOffset _maskoffset)
      (Variables|MaterialSettings|SetGraffitiOffset _graffitioffset)
      (Variables|MaterialSettings|SetGraffitiUVScale _graffitiuvscale)
      (Variables|MaterialSettings|SetRoughness _roughness)
      (Variables|MaterialSettings|SetMetallic _metallic))
    (:then_1
      (MaterialSettings|UpdateGraffitiDecal))))

(fn RandomizeColor
  (Utilities|FlowControl|Sequence
    (:then_0
      (Variables|MaterialSettings|SetHueShift (Math|Random|RandomFloatinRange 0.0 1.0))
      (Variables|MaterialSettings|SetDesaturation (Math|Random|RandomFloatinRange 0.0 1.0))
      (Variables|MaterialSettings|SetBrightness (Math|Random|RandomFloatinRange 0.5 1.0))
      (Variables|MaterialSettings|SetColorMultiply "(R=1.000000,G=1.000000,B=1.000000,A=1.000000)"))
    (:then_1
      (MaterialSettings|UpdateGraffitiDecal))))

(fn RandomizeGraffiti
  (bind _outassetdata (Class|AssetRegistry|GetAssetsbyPath (Class|AssetRegistryHelpers|GetAssetRegistry) (Variables|MaterialSettings|GetGraffitiPath) true false))
  (bind _astexture_2d (Utilities|Casting|CastToTexture2D (Class|AssetRegistryHelpers|GetAsset (Utilities|Array|Get(acopy) _outassetdata (Math|Random|RandomIntegerinRange 0 (Utilities|Array|LastIndex _outassetdata))))))
  (Variables|MaterialSettings|SetGraffitiTexture _astexture_2d)
  (MaterialSettings|UpdateGraffitiDecal))